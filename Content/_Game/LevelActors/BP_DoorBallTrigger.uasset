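; BP_DoorBallTrigger is a door actor that toggles open and closed when struck by a BP_FirstPersonBlastBall or triggered through Interact.
; Hits on Box count only when DirectHitTrigger is set, while Box1 hits and Interact always toggle.
; A FlipFlop alternately plays and reverses a timeline that slides the Cube vertically.
; With OneTime set, the actor destroys itself when the timeline finishes.
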(event `self.Box.OnComponentHit`
  (params (HitComponent :type "PrimitiveComponent Object Reference") (OtherActor :type "Actor Object Reference") (OtherComp :type "PrimitiveComponent Object Reference") (NormalImpulse :type "Vector Structure") (Hit :type "HitResult Structure (by ref)"))
  (cast `/Game/FirstPerson/Blueprints/BP_FirstPersonBlastBall` OtherActor)
  (if (`self.DirectHitTrigger?`)
    (`/Engine/EditorBlueprintResources/StandardMacros.FlipFlop` :!label _label
      (:`A`
        (bind (_direction _doortrack) (`Timeline|Open/Close Door Timeline` :!label _label_2)
          (:`Update`
            (`SceneComponent.K2_SetRelativeLocation` (`self.Cube`) (`KismetMathLibrary.MakeVector` 0.0 0.0 (`KismetMathLibrary.Lerp` 100.0 -110.0 _doortrack)) false false))
          (:`Finished`
            (if (`self.OneTime?`)
              (`self.K2_DestroyActor`)))))
      (:`B`
        (goto _label_2 :!via `Reverse`)))))

(event `self.Box1.OnComponentHit`
  (params (HitComponent :type "PrimitiveComponent Object Reference") (OtherActor :type "Actor Object Reference") (OtherComp :type "PrimitiveComponent Object Reference") (NormalImpulse :type "Vector Structure") (Hit :type "HitResult Structure (by ref)"))
  (cast `/Game/FirstPerson/Blueprints/BP_FirstPersonBlastBall` OtherActor)
  (goto _label))

(event `/Game/_Game/InteractInterface.Interact`
  (goto _label))

(fn `UserConstructionScript`)
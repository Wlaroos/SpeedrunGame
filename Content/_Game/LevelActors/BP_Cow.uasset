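; BP_Cow is a level actor cow that explodes into meat and blood the first time it is interacted with.
; Interact hides the body, launches three BP_MeatChunk actors with random impulses, spawns explosion effects and sound at the hit location, and calls Win.
; The particle system receives the cow as its callback object, so ParticleData places randomized, fading blood decals at exported particle positions, oriented against their velocity.
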(event `/Game/_Game/InteractInterface.Interact`
  (params (HitLoc :type "Vector Structure"))
  (bind _cow_body (`self.Cow_Body`))
  (bind (_returnvalue_x _returnvalue_y _returnvalue_z) (`KismetMathLibrary.BreakVector` (`SceneComponent.K2_GetComponentLocation` _cow_body)))
  (`/Engine/EditorBlueprintResources/StandardMacros.DoOnce` false
    (:`Completed`
      (`SceneComponent.SetVisibility` _cow_body false false)
      (for _index (range 3)
        (bind _returnvalue (`|SpawnActorFromClass` "/Game/_Game/LevelActors/BP_MeatChunk.BP_MeatChunk_C" (`KismetMathLibrary.MakeTransform` (`KismetMathLibrary.MakeVector` _returnvalue_x (+ (- _returnvalue_y 50.0) (* _index 75)) (+ _returnvalue_z 10.0))) "Undefined" "MultiplyWithRoot" null null))
        (`PrimitiveComponent.AddImpulse` (`/Game/_Game/LevelActors/BP_MeatChunk.MeatChunk_Mesh` _returnvalue) (`KismetMathLibrary.MakeVector` (`KismetMathLibrary.RandomFloatInRange` -200.0 200.0) (`KismetMathLibrary.RandomFloatInRange` -200.0 200.0) (`KismetMathLibrary.RandomFloatInRange` 333.0 500.0)) "None" true))
      (bind _returnvalue_2 (`NiagaraFunctionLibrary.SpawnSystemAtLocation` "/Game/_Game/Particles/PS_CowExplode.PS_CowExplode" HitLoc))
      (`NiagaraComponent.SetVariableObject` _returnvalue_2 "BP_Blood" self)
      (bind _returnvalue_3 (`GameplayStatics.SpawnSoundAtLocation` "/Game/_Game/SFX/CowExplode_Cue.CowExplode_Cue" HitLoc (struct) 1.0 1.0 0.0 null null))
      (`self.Win` _returnvalue_3))))

(event `self.ReceiveParticleData`
  (params (Data :type "Array of BasicParticleData Structure (by ref)") (NiagaraSystem :type "NiagaraSystem Object Reference") (SimulationPositionOffset :type "Vector Structure (by ref)"))
  (bind _returnvalue (`KismetMathLibrary.RandomFloatInRange` 15.0 50.0))
  (for _array_element Data
    (bind (_position _size _velocity) (break `BasicParticleData` _array_element))
    (bind _returnvalue_2 (`GameplayStatics.SpawnDecalAtLocation` (select `int` (`KismetMathLibrary.RandomInteger` 2) :`0` "/Game/_Game/Decals/M_BloodDecal01.M_BloodDecal01" :`1` "/Game/_Game/Decals/M_BloodDecal02.M_BloodDecal02" :`2` "/Game/_Game/Decals/M_BloodDecal03.M_BloodDecal03" :!type "MaterialInterface Object Reference") (`KismetMathLibrary.MakeVector` _returnvalue _returnvalue _returnvalue) _position (`KismetMathLibrary.Conv_VectorToRotator` (* _velocity -1.0))))
    (`DecalComponent.SetFadeOut` _returnvalue_2 2.0 3.0 true)))

(fn `UserConstructionScript`)
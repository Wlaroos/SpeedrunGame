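; Breakable board actor that snaps into two loose pieces when the player interacts with it.
; Interact runs Break only once, destroying the intact Cube, then revealing Cube1 and Cube2 and enabling their physics.
; Both pieces get a mass-independent impulse along the first-person camera's forward vector, using the player character reference cached on BeginPlay.
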(event `/Game/_Game/InteractInterface.Interact`
  (`/Engine/EditorBlueprintResources/StandardMacros.DoOnce` false
    (:`Completed`
      (`self.Break`))))

(event `Break`
  (bind _cube2 (`self.Cube2`))
  (bind _cube1 (`self.Cube1`))
  (bind _firstpersoncamera (`/Game/FirstPerson/Blueprints/BP_FirstPersonCharacter.FirstPersonCamera` (`self.PlayerRef`)))
  (bind _returnvalue (`SceneComponent.K2_GetComponentLocation` _firstpersoncamera))
  (bind _returnvalue_2 (* (- (+ _returnvalue (* (`KismetMathLibrary.GetForwardVector` (`SceneComponent.K2_GetComponentRotation` _firstpersoncamera)) 100.0)) _returnvalue) 5.0))
  (`ActorComponent.K2_DestroyComponent` (`self.Cube`))
  (`SceneComponent.SetVisibility` _cube1 true false)
  (`SceneComponent.SetVisibility` _cube2 true false)
  (`PrimitiveComponent.SetSimulatePhysics` _cube1 true)
  (`PrimitiveComponent.SetSimulatePhysics` _cube2 true)
  (`PrimitiveComponent.AddImpulse` (`self.Cube1`) _returnvalue_2 "None" true)
  (`PrimitiveComponent.AddImpulse` (`self.Cube2`) _returnvalue_2 "None" true))

(event `self.ReceiveBeginPlay`
  (bind _asbp_first_person_character (cast `/Game/FirstPerson/Blueprints/BP_FirstPersonCharacter` (`GameplayStatics.GetPlayerCharacter` 0)))
  (set `self.PlayerRef` _asbp_first_person_character))

(fn `UserConstructionScript`)
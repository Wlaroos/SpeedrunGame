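; Short breakable wooden board that snaps into two physics pieces when the player interacts with it.
; Interact fires once, hiding the intact plank, disabling its collision and revealing the two pieces hidden at BeginPlay.
; Both pieces get a mass-independent impulse along the first-person camera's forward vector, and a plank-break particle system spawns at the hit location.
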(event `/Game/_Game/InteractInterface.Interact`
  (params (HitLoc :type "Vector Structure"))
  (`/Engine/EditorBlueprintResources/StandardMacros.DoOnce` false
    (:`Completed`
      (`self.Break` HitLoc))))

(event `self.ReceiveBeginPlay`
  (bind _asbp_first_person_character (cast `/Game/FirstPerson/Blueprints/BP_FirstPersonCharacter` (`GameplayStatics.GetPlayerCharacter` 0)))
  (set `self.PlayerRef` _asbp_first_person_character)
  (`SceneComponent.SetVisibility` (`self.M_PlankPiece01`) false false)
  (`SceneComponent.SetVisibility` (`self.M_PlankPiece02`) false false))

(event `Break`
  (params (HitLoc :type "Vector Structure"))
  (bind _m_plank (`self.M_Plank`))
  (bind _m_plankpiece02 (`self.M_PlankPiece02`))
  (bind _m_plankpiece01 (`self.M_PlankPiece01`))
  (bind _firstpersoncamera (`/Game/FirstPerson/Blueprints/BP_FirstPersonCharacter.FirstPersonCamera` (`self.PlayerRef`)))
  (bind _returnvalue (`SceneComponent.K2_GetComponentLocation` _firstpersoncamera))
  (bind _returnvalue_2 (* (- (+ _returnvalue (* (`KismetMathLibrary.GetForwardVector` (`SceneComponent.K2_GetComponentRotation` _firstpersoncamera)) 100.0)) _returnvalue) 5.0))
  ;[1 1 1] Comment
  (`SceneComponent.SetVisibility` _m_plank false false)
  (`PrimitiveComponent.SetCollisionEnabled` _m_plank "NoCollision")
  (`SceneComponent.SetVisibility` _m_plankpiece01 true false)
  (`SceneComponent.SetVisibility` _m_plankpiece02 true false)
  (`PrimitiveComponent.SetSimulatePhysics` _m_plankpiece01 true)
  (`PrimitiveComponent.SetSimulatePhysics` _m_plankpiece02 true)
  (`PrimitiveComponent.AddImpulse` _m_plankpiece01 _returnvalue_2 "None" true)
  (`PrimitiveComponent.AddImpulse` _m_plankpiece02 _returnvalue_2 "None" true)
  (`NiagaraFunctionLibrary.SpawnSystemAtLocation` "/Game/_Game/Particles/PS_PlankBreak.PS_PlankBreak" HitLoc))

(fn `UserConstructionScript`)